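; Enemy actor Blueprint that tracks its own health and removes itself from the game when that health runs out.
; BeginPlay initializes Hp, and the DecreaseHP event subtracts the given amount.
; At zero or below, it destroys the actor, then calls SubCnt on the ShooterGameMode to report the loss.
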(event `self.ReceiveBeginPlay`
  (set `self.hp` 100.0))

(event `/Game/DamageInterface.DecreaseHP`
  (params (Amount :type "Float (single-precision)"))
  (bind _output_get (set `self.hp` (- (`self.hp`) Amount)))
  (if (<= _output_get 0.0)
    (`self.K2_DestroyActor`)
    (bind _asshooter_game_mode (cast `/Game/ShooterGameMode` (`GameplayStatics.GetGameMode`)))
    (`/Game/ShooterGameMode.Sub Cnt` _asshooter_game_mode)))

(fn `UserConstructionScript`)