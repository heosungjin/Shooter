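; Enemy2BP is an enemy actor that damages the hero on contact and can be killed.
; On overlap with HeroBP it deals damage at once and sets a non-looping timer for one follow-up hit, cleared if the hero leaves first.
; Its DecreaseHP event lowers its own health and, at zero, destroys the actor and calls SubCnt on ShooterGameMode.
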(event `/Game/DamageInterface.DecreaseHP`
  (params (Amount :type "Float (single-precision)"))
  (bind _output_get (set `self.HP` (- (`self.HP`) Amount)))
  (if (<= _output_get 0.0)
    (`self.K2_DestroyActor`)
    (bind _asshooter_game_mode (cast `/Game/ShooterGameMode` (`GameplayStatics.GetGameMode`)))
    (`/Game/ShooterGameMode.Sub Cnt` _asshooter_game_mode)))

(event `self.ReceiveBeginPlay`
  (set `self.HP` 100.0))

(event `self.ReceiveActorBeginOverlap`
  (params (OtherActor :type "Actor Object Reference"))
  (bind _ashero_bp (cast `/Game/Hero/HeroBP` OtherActor))
  (if true
    (bind _output_get (set `self.hero` _ashero_bp))
    (message `/Game/DamageInterface.DecreaseHP` _output_get 30.0)
    (`KismetSystemLibrary.K2_SetTimer` null "HeroDHP" 1.0)))

(event `HeroDHP`
  (message `/Game/DamageInterface.DecreaseHP` (`self.hero`) 30.0))

(event `self.ReceiveActorEndOverlap`
  (params (OtherActor :type "Actor Object Reference"))
  (if (== OtherActor (`self.hero`))
    (`KismetSystemLibrary.K2_ClearTimer` null "HeroDHP")))

(fn `UserConstructionScript`)