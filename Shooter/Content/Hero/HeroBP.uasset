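; HeroBP is the player hero, spawning a gun and handling movement and turning input.
; On BeginPlay it spawns a GunBP, stores it and snaps it to the mesh's hand_r socket.
; Forward and right axes feed movement input along fixed world X and Y directions, independent of facing.
; A separate Turn Right axis rotates the actor's local yaw, scaled by the axis value.
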(event `self.ReceiveBeginPlay`
  (bind _returnvalue (`|SpawnActorFromClass` "/Game/Gun/GunBP.GunBP_C" (`SceneComponent.K2_GetComponentToWorld` (`self.Mesh`)) "Undefined" "OverrideRootScale"))
  (bind _output_get (set `self.Gun` _returnvalue))
  (`self.K2_AttachToComponent` _output_get (`self.Mesh`) "hand_r" "SnapToTarget" "SnapToTarget" "KeepRelative" true))

(event `InputAxis|Move Forward`
  (params (AxisValue :type "Float (single-precision)"))
  (`self.AddMovementInput` (5.0 0.0 0.0) AxisValue))

(event `InputAxis|Move Right`
  (params (AxisValue :type "Float (single-precision)"))
  (`self.AddMovementInput` (0.0 5.0 0.0) AxisValue))

(event `InputAxis|Turn Right`
  (params (AxisValue :type "Float (single-precision)"))
  (`self.K2_AddActorLocalRotation` (`KismetMathLibrary.MakeRotator` 0.0 0.0 (* AxisValue 2.0))))

(fn `UserConstructionScript`)